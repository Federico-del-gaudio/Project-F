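; Weapon actor for the player, configured through GunData for mesh, offsets, stats, effects and sounds.
; PullTrigger plays a camera shake and switches on fire mode, where hitscan adds recoil, muzzle effects and a camera-based line trace with persistent debug drawing.
; Hits spawn impacts and sounds, and Enemy-tagged actors receive crit-rolled damage with gameplay tags via TakeDamageMessage.
; Tick applies interpolated recoil recovery and speed-scaled sine bobbing to the mesh.
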(event `self.ReceiveTick`
  (params (DeltaSeconds :type "Float (single-precision)"))
  (bind _weapon (`self.Weapon`))
  (bind _returnvalue (`KismetMathLibrary.RInterpTo` (`self.CurrentRecoilRotation`) (struct) DeltaSeconds 5.0))
  (bind (_bobintensity _bobbingspeed) (break `/Game/WeaponClass/S_FWeaponRecoil` (`/Game/GunData/DA_WeaponData.WeaponBob` (`self.GunData`))))
  ; Recoil e bobbing
  (`|ExecutionSequence`
    (:`then_0`
      (set `self.CurrentRecoilLocation` (+ (`self.RecoilRestPosition`) (`KismetMathLibrary.VInterpTo` (`self.CurrentRecoilLocation`) (0.0 0.0 0.0) DeltaSeconds 5.0)))
      (set `self.CurrentRecoilRotation` _returnvalue)
      (`SceneComponent.K2_SetRelativeLocation` _weapon (+ (`self.RecoilRestPosition`) (`KismetMathLibrary.MakeVector` 0.0 0.0 (* (* _bobintensity (`KismetMathLibrary.Sin` (`self.BobTimer`))) (+ (/ (`KismetMathLibrary.VSize` (`self.GetVelocity` (`GameplayStatics.GetPlayerCharacter` 0))) 1150.0) 0.2)))) false false)
      (`SceneComponent.K2_SetRelativeRotation` _weapon (`KismetMathLibrary.ComposeRotators` _returnvalue (`self.RecoilRestRotation`)) false false))
    (:`then_1`
      (set `self.BobTimer` (+ (`self.BobTimer`) (* _bobbingspeed (`GameplayStatics.GetWorldDeltaSeconds`)))))))

(event `self.ReceiveBeginPlay`
  (bind (_relativeoffsett_location _relativeoffsett_rotation) (`KismetMathLibrary.BreakTransform` (`/Game/GunData/DA_WeaponData.RelativeOffsett` (`self.GunData`))))
  (bind (_relativeoffsett_location_2 _relativeoffsett_rotation_2 _relativeoffsett_scale) (`KismetMathLibrary.BreakTransform` (`/Game/GunData/DA_WeaponData.RelativeOffsett` (`self.GunData`))))
  (`StaticMeshComponent.SetStaticMesh` (`self.Weapon`) (`/Game/GunData/DA_WeaponData.Weapon Mesh` (`self.GunData`)))
  (set `self.RecoilRestPosition` _relativeoffsett_location)
  (set `self.RecoilRestRotation` _relativeoffsett_rotation)
  (`|SwitchGameplayTag` (`self.HandTag`)
    (:`Default`
      (`SceneComponent.SetRelativeScale3D` (`self.Weapon`) _relativeoffsett_scale)
      (`SceneComponent.K2_SetRelativeRotation` (`self.Weapon`) _relativeoffsett_rotation_2 false false))
    (:`Case_0`
      (`SceneComponent.K2_SetRelativeLocation` (`self.Weapon`) (0.0 0.0 0.0) false false))
    (:`Case_1`
      (`SceneComponent.K2_SetRelativeLocation` (`self.Weapon`) (0.0 0.0 0.0) false false))))

(event `Hitscan`
  (`self.SpawnMuzzleFX` (struct))
  (`self.ApplyRecoil`)
  (`self.HitScanLogic`))

(fn `ApplyDetectionSound`
  (params (SoundLocation :type "Vector Structure") (HitResult :type "HitResult Structure") (Weapon :type "/Game/WeaponClass/BP_WeaponClass Object Reference") (`Impact Tags` :type "GameplayTagContainer Structure"))
  (bind (_bblockinghit _binitialoverlap _time _distance _location _impactpoint _normal _impactnormal _physmat _hitactor) (`GameplayStatics.BreakHitResult` HitResult))
  (bind (_shootsound _impactsound _enemyimpactsound _critsound) (break `/Game/WeaponClass/S_WeaponAudios` (`/Game/GunData/DA_WeaponData.WeaponSounds` (`self.GunData`))))
  (`/Engine/EditorBlueprintResources/StandardMacros.IsValid` _hitactor
    (:`Is Valid`
      (`GameplayStatics.PlaySoundAtLocation` (select `bool` (`BlueprintGameplayTagLibrary.HasTag` `Impact Tags` (struct :`TagName` "Damage.Effect.Critical") true) :`false` (select `bool` (`self.ActorHasTag` _hitactor "Enemy") :`false` _impactsound :`true` _enemyimpactsound) :`true` _critsound) SoundLocation (struct) 1.0 1.0 0.0 null null null null))))

(fn `ApplyRecoil`
  (bind (_recoilcurve _recoilrotation _recoillocation) (break `/Game/WeaponClass/S_FWeaponMovement` (`/Game/GunData/DA_WeaponData.WeaponRecoil` (`self.GunData`))))
  (set `self.CurrentRecoilLocation` (+ _recoillocation (`self.CurrentRecoilLocation`)))
  (set `self.CurrentRecoilRotation` (`KismetMathLibrary.ComposeRotators` _recoilrotation (`self.CurrentRecoilRotation`))))

(fn `ApplyShootingSound`
  (params (SoundLocation :type "Vector Structure") (HitResult :type "HitResult Structure") (Weapon :type "/Game/WeaponClass/BP_WeaponClass Object Reference") (`Impact Tags` :type "GameplayTagContainer Structure"))
  (`|ExecutionSequence`
    (:`then_0`
      (`GameplayStatics.PlaySoundAtLocation` (`.ShootSound_19_F9762E47424836A6B4519B8316A55651` (break `/Game/WeaponClass/S_WeaponAudios` (`/Game/GunData/DA_WeaponData.WeaponSounds` (`self.GunData`)))) (`self.K2_GetActorLocation` Weapon) (struct) 1.0 1.0 0.0 null null null null))))

(fn `Calculate Damage`
  (params (HitResult :type "HitResult Structure") (`Damage Direction` :type "Vector Structure"))
  (returns (`Final Damage` :type "Float (double-precision)") (`Out Tags` :type "GameplayTagContainer Structure"))
  (locals (LocalDamage :type "Float (double-precision)") (LocalTags :type "GameplayTagContainer Structure"))
  (bind _gundata (`self.GunData`))
  (bind _damage (`/Game/GunData/DA_WeaponData.Damage` _gundata))
  (set `local.LocalTags` (struct))
  (if (<= (`KismetMathLibrary.RandomFloatInRange` 0.0 100.0) (`/Game/GunData/DA_WeaponData.Crit Chance` _gundata))
    (`BlueprintGameplayTagLibrary.AddGameplayTag` (`local.LocalTags`) (struct :`TagName` "Damage.Effect.Critical"))
    (set `local.LocalDamage` (* _damage (`/Game/GunData/DA_WeaponData.Crit Damage` _gundata)))
    (else
      (set `local.LocalDamage` _damage)
      (set `local.LocalTags` (struct))))
  (return (`local.LocalDamage`) (`local.LocalTags`)))

(fn `HitScanLogic`
  (returns (HitResult :type "HitResult Structure"))
  (bind _returnvalue (`GameplayStatics.GetPlayerCameraManager` 0))
  (bind _out_hit (`self.Out Hit`))
  (bind _returnvalue_2 (`PlayerCameraManager.GetCameraLocation` _returnvalue))
  (bind (_outhit _returnvalue_3) (`KismetSystemLibrary.LineTraceSingle` :`Start` _returnvalue_2 :`End` (+ _returnvalue_2 (* (`KismetMathLibrary.GetForwardVector` (`PlayerCameraManager.GetCameraRotation` _returnvalue)) (`/Game/GunData/DA_WeaponData.Range` (`self.GunData`)))) :`TraceChannel` "TraceTypeQuery1" :`DrawDebugType` "Persistent"))
  (bind _output_get (set `self.Out Hit` _outhit))
  (bind (_bblockinghit _binitialoverlap _time _distance _location _impactpoint _normal _impactnormal _physmat _hitactor) (`GameplayStatics.BreakHitResult` _outhit))
  (`self.SpawnTraceFX` _impactpoint)
  (`self.ApplyShootingSound` (0.0 0.0 0.0) _output_get self)
  (if _returnvalue_3
    (`self.SpawnImpact` _out_hit)
    (if (`self.ActorHasTag` _hitactor "Enemy")
      (bind (_final_damage _out_tags) (`self.Calculate Damage` (struct)))
      (bind _output_get_2 (set `self.Out Tags` _out_tags))
      (message `/Game/DamageableActors/BPI_Damageable.TakeDamage` _hitactor _final_damage _output_get_2 _out_hit (`GameplayStatics.GetPlayerCharacter` 0))
      (else
        (set `self.Out Tags` (struct))))
    (`self.ApplyDetectionSound` _impactpoint (`self.Out Hit`) self (`self.Out Tags`))
    (return (`self.Out Hit`))))

(fn `PullTrigger`
  (`PlayerController.ClientStartCameraShake` :`self` (`GameplayStatics.GetPlayerController` 0) :`Shake` (`/Game/GunData/DA_WeaponData.ShootCameraShake` (`self.GunData`)) :`PlaySpace` "World")
  (`|SwitchGameplayTag` (`/Game/GunData/DA_WeaponData.Fire Mode Tag` (`self.GunData`))
    (:`HitScan`
      (`self.Hitscan`))))

(fn `SpawnImpact`
  (params (HitResult :type "HitResult Structure"))
  (bind (_bblockinghit _binitialoverlap _time _distance _location _impactpoint _normal _impactnormal) (`GameplayStatics.BreakHitResult` HitResult))
  (`NiagaraFunctionLibrary.SpawnSystemAtLocation` (`.ImpactEffect_7_290764E74ABDEFB2C18817BAF91D8DAE` (break `/Game/WeaponClass/S_FWeaponFX` (`/Game/GunData/DA_WeaponData.WeaponFX` (`self.GunData`)))) _impactpoint (`KismetMathLibrary.MakeRotFromX` _impactnormal)))

(fn `SpawnMuzzleFX`
  (params (HitResult :type "HitResult Structure"))
  (bind (_muzzleflash _tracersystem _impacteffect _muzzlesocketnames) (break `/Game/WeaponClass/S_FWeaponFX` (`/Game/GunData/DA_WeaponData.WeaponFX` (`self.GunData`))))
  (for _array_element _muzzlesocketnames
    (`NiagaraFunctionLibrary.SpawnSystemAttached` _muzzleflash (`self.Weapon`) _array_element (0.0 0.0 0.0) (struct) "SnapToTarget")))

(fn `SpawnTraceFX`
  (params (EndLocation :type "Vector Structure"))
  (bind (_muzzleflash _tracersystem _impacteffect _muzzlesocketnames) (break `/Game/WeaponClass/S_FWeaponFX` (`/Game/GunData/DA_WeaponData.WeaponFX` (`self.GunData`))))
  (for _array_element _muzzlesocketnames
    (bind _returnvalue (`NiagaraFunctionLibrary.SpawnSystemAttached` _tracersystem (`self.Weapon`) _array_element (0.0 0.0 0.0) (struct) "KeepRelativeOffset" true true "ManualRelease"))
    (`NiagaraComponent.SetNiagaraVariableVec3` _returnvalue "start" (`SceneComponent.GetSocketLocation` (`self.Weapon`) _array_element))
    (`NiagaraComponent.SetNiagaraVariableVec3` _returnvalue "end" EndLocation)))

(fn `UserConstructionScript`)